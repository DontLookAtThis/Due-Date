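; BP_Small_Box_Bin is a sorting bin that scores small box parcels dropped into it.
; When a non-player actor overlaps its Box, a class cast checks for BP_Parcel_Small_box.
; Either way it destroys the actor and releases the player's PhysicsHandle grab.
; It then tells BP_GameMode to increase the score for a small box or decrease it for anything else.
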(event OnComponentBeginOverlap(Box)
  (params (OverlappedComponent :type Primitive%20Component%20Object%20Reference) (OtherActor :type Actor%20Object%20Reference) (OtherComp :type Primitive%20Component%20Object%20Reference) (OtherBodyIndex :type Integer) (bFromSweep :type Boolean) (SweepResult :type Hit%20Result%20Structure%20%28by%20ref%29))
  (bind _output_get (Variables|Default|SetOther%20Actor OtherActor))
  (Utilities|Casting|CastToBP_Player _output_get
    (:CastFailed
      (Utilities|Casting|CastToBP_Parcel_Small_boxClass (Utilities|GetClass _output_get)
        (:then
          (Actor|DestroyActor (Variables|Default|GetOther%20Actor))
          (bind _asbp_player (Utilities|Casting|CastToBP_Player (Game|Player|GetPlayerPawn 0)))
          (Physics|Components|PhysicsHandle|ReleaseComponent (Variables|/Game/Player_Assets/BP_Player.BP_Player_C|GetPhysicsHandle _asbp_player))
          (bind _asbp_game_mode (Utilities|Casting|CastToBP_GameMode (Game|GetGameMode)))
          (Default|IncreaseScore _asbp_game_mode))
        (:CastFailed
          (Actor|DestroyActor (Variables|Default|GetOther%20Actor))
          (bind _asbp_player_2 (Utilities|Casting|CastToBP_Player (Game|Player|GetPlayerPawn 0)))
          (Physics|Components|PhysicsHandle|ReleaseComponent (Variables|/Game/Player_Assets/BP_Player.BP_Player_C|GetPhysicsHandle _asbp_player_2))
          (bind _asbp_game_mode_2 (Utilities|Casting|CastToBP_GameMode (Game|GetGameMode)))
          (Default|DecreaseScore _asbp_game_mode_2))))))

(event EventBeginPlay)

(event Collision|EventActorBeginOverlap
  (params (OtherActor :type Actor%20Object%20Reference)))

(event EventTick
  (params (DeltaSeconds :type Float%20%28single-precision%29)))

(fn ConstructionScript)