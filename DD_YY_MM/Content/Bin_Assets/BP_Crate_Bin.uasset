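; BP_Crate_Bin is a parcel drop-off bin that scores the player for receiving crate parcels.
; Its Box overlap ignores the player, destroys any other actor, releases the player's PhysicsHandle and raises the GameMode score for BP_Parcel_Crate, otherwise lowers it.
; A Cone marker bobs on a sine in Tick while Activated.
; Activate toggles that flag and Cone visibility, although BeginPlay sets the flag true with the Cone hidden.
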(event OnComponentBeginOverlap(Box)
  (params (OverlappedComponent :type Primitive%20Component%20Object%20Reference) (OtherActor :type Actor%20Object%20Reference) (OtherComp :type Primitive%20Component%20Object%20Reference) (OtherBodyIndex :type Integer) (bFromSweep :type Boolean) (SweepResult :type Hit%20Result%20Structure%20%28by%20ref%29))
  (bind _output_get (Variables|Default|SetOther%20Actor OtherActor))
  (Utilities|Casting|CastToBP_Player _output_get ; Ignoring the collision if it is the player
    (:CastFailed
      (Utilities|Casting|CastToBP_Parcel_CrateClass (Utilities|GetClass _output_get) ; casting to the crate class
        (:then
          ;[1 1 1] Correct parcel type was passed in
          (Actor|DestroyActor (Variables|Default|GetOther%20Actor))
          (bind _asbp_player (Utilities|Casting|CastToBP_Player (Game|Player|GetPlayerPawn 0)))
          (Physics|Components|PhysicsHandle|ReleaseComponent (Variables|/Game/Player_Assets/BP_Player.BP_Player_C|GetPhysicsHandle _asbp_player))
          (bind _asbp_game_mode (Utilities|Casting|CastToBP_GameMode (Game|GetGameMode)))
          (Default|IncreaseScore _asbp_game_mode))
        (:CastFailed
          ;[1 1 1] Incorrect parcel type was passed in
          (Actor|DestroyActor (Variables|Default|GetOther%20Actor))
          (bind _asbp_player_2 (Utilities|Casting|CastToBP_Player (Game|Player|GetPlayerPawn 0)))
          (Physics|Components|PhysicsHandle|ReleaseComponent (Variables|/Game/Player_Assets/BP_Player.BP_Player_C|GetPhysicsHandle _asbp_player_2))
          (bind _asbp_game_mode_2 (Utilities|Casting|CastToBP_GameMode (Game|GetGameMode)))
          (Default|DecreaseScore _asbp_game_mode_2))))))

(event EventBeginPlay
  (Variables|Default|SetActivated true)
  (Rendering|SetVisibility (Variables|Default|GetCone) false false))

(event Collision|EventActorBeginOverlap
  (params (OtherActor :type Actor%20Object%20Reference)))

(event EventTick
  (params (DeltaSeconds :type Float%20%28single-precision%29))
  (bind _cone (Variables|Default|GetCone))
  (if (Variables|Default|GetActivated)
    (bind _output_get (Variables|Default|SetBobbing (+ (Variables|Default|GetBobbing) 3)))
    (Transformation|SetRelativeLocation _cone (+ (Variables|/Script/Engine.SceneComponent|GetRelativeLocation _cone) (Math|Vector|MakeVector 0.0 0.0 (* (Math|Trig|Sin(Degrees) (Math|Conversions|ToFloat(Integer) _output_get)) 5.0))) false false)))

(fn ConstructionScript)

(fn Activate
  (bind _output_get (Variables|Default|SetActivated (not (Variables|Default|GetActivated))))
  (Rendering|SetVisibility (Variables|Default|GetCone) _output_get false)
  (return))