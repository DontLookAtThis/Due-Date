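; Game mode for Due_Date that runs the level countdown and opens the Game_Over level when time expires.
; BeginPlay seeds Minute and Seconds, and Tick uses a one-second Delay as a throttle to count them down, rolling minutes over and setting TimeUp at zero.
; Each step rebuilds the zero-padded Time string, though the colon is only appended when minutes are below ten.
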(event EventBeginPlay
  (Actor|Tick|SetActorTickEnabled true)
  (Variables|Default|SetSeconds 14)
  (Variables|Default|SetMinute 0))

(event EventTick
  (params (DeltaSeconds :type Float%20%28single-precision%29))
  (Utilities|FlowControl|Delay 1.0)
  (if (== (Variables|Default|GetSeconds) 0)
    (if (== (Variables|Default|GetMinute) 0)
      (Variables|Default|SetTimeUp true)
      (Game|OpenLevel(byName) "Game_Over")
      (else
        (Variables|Default|SetMinute (- (Variables|Default|GetMinute) 1))
        (Variables|Default|SetSeconds 59)
        (if (<= (Variables|Default|GetMinute) 9) :!label _label ; If there are less than 10m
          (Variables|Default|SetTime (Utilities|String|Append "0" (Utilities|String|ToString(Integer) (Variables|Default|GetMinute)) ":"))
          (else
            (Variables|Default|SetTime (Utilities|String|ToString(Integer) (Variables|Default|GetMinute)))))
        (if (<= (Variables|Default|GetSeconds) 9) ; If there are less that 10s
          (Variables|Default|SetTime (Utilities|String|Append (Variables|Default|GetTime) "0" (Utilities|String|ToString(Integer) (Variables|Default|GetSeconds))))
          (else
            (Variables|Default|SetTime (Utilities|String|Append (Variables|Default|GetTime) (Utilities|String|ToString(Integer) (Variables|Default|GetSeconds))))))))
    (else
      (Variables|Default|SetSeconds (- (Variables|Default|GetSeconds) 1))
      (goto _label))))

(fn ConstructionScript)